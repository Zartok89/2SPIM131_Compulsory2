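; Player character Blueprint for the PKRPG game, handling experience gain and a keyboard-triggered health loss.
; On BeginPlay it binds to the OnEnemyDeath dispatcher and adds a fixed amount to CharacterExp in PKAttributeData on each enemy death.
; Pressing Q broadcasts OnHealthLost with a fixed amount, then destroys the actor if Health in PKAttributeData is zero or below.
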(event `self.ReceiveBeginPlay`
  (add `PKCharacter.OnEnemyDeath` (delegate `OnEnemyDeath_Event`)))

(event `OnEnemyDeath_Event`
  (params (Character :type "PKCharacter Object Reference"))
  (bind _pkattributedata (`self.PKAttributeData`))
  (set `PKAttributeDataComponent.CharacterExp` (+ (`PKAttributeDataComponent.CharacterExp` _pkattributedata) 5) _pkattributedata))

(event `self.ReceiveTick`
  (params (DeltaSeconds :type "Float (single-precision)")))

(event `Key|Q`
  (params (Key :type "Key Structure"))
  (:`Pressed`
    (`self.OnHealthLost` 25.0)
    (if (<= (`PKAttributeDataComponent.Health` (`self.PKAttributeData`)) 0.0)
      (`self.K2_DestroyActor`))))

(fn `UserConstructionScript`)