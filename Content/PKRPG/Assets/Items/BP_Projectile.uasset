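; BP_Projectile is a projectile actor that plays a sound when spawned and destroys itself after ten seconds.
; When its sphere overlaps an actor of exactly the BP_NPC class, it calls CallOnEnemyHit with that NPC's attribute data.
; It then clears the NPC's mesh, attaches an explosion effect with sound, destroys itself and disables the NPC's collision, leaving the NPC actor undestroyed.
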(event `self.ReceiveBeginPlay`
  (`GameplayStatics.PlaySound2D` "/Engine/VREditor/Sounds/UI/Floating_UI_Open-002.Floating_UI_Open-002" 3.0 1.0 0.0 null null)
  (`KismetSystemLibrary.Delay` 10.0)
  (`self.K2_DestroyActor`))

(event `self.Sphere.OnComponentBeginOverlap`
  (params (OverlappedComponent :type "PrimitiveComponent Object Reference") (OtherActor :type "Actor Object Reference") (OtherComp :type "PrimitiveComponent Object Reference") (OtherBodyIndex :type Integer) (bFromSweep :type Boolean) (SweepResult :type "HitResult Structure (by ref)"))
  (if (== (`GameplayStatics.GetObjectClass` OtherActor) "/Game/PKRPG/Assets/Characters/NPC/BP_NPC.BP_NPC_C")
    (bind _asbp_npc (cast `/Game/PKRPG/Assets/Characters/NPC/BP_NPC` OtherActor))
    (`self.OnEnemyHit` (`/Game/PKRPG/Assets/Characters/NPC/BP_NPC.PKAttributeData` _asbp_npc))
    (bind _staticmesh (`/Game/PKRPG/Assets/Characters/NPC/BP_NPC.StaticMesh` _asbp_npc))
    (`StaticMeshComponent.SetStaticMesh` _staticmesh null)
    (`NiagaraFunctionLibrary.SpawnSystemAttached` "/Niagara/DefaultAssets/Templates/Systems/SimpleExplosion.SimpleExplosion" _staticmesh "None" (0.0 0.0 0.0) (struct) "SnapToTarget" true)
    (`GameplayStatics.PlaySound2D` "/Game/PKRPG/Assets/Audio/Explosion+1.Explosion+1" 3.0 1.0 0.0 null null)
    (`self.K2_DestroyActor`)
    (`self.SetActorEnableCollision` _asbp_npc false)))

(fn `UserConstructionScript`)