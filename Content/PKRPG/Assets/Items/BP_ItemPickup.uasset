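; BP_ItemPickup is an item pickup actor that displays its item name and is collected when the player touches it.
; On BeginPlay it writes the item name to its text display.
; When an actor tagged Player overlaps its sphere, it broadcasts the OnItemPickup dispatcher with the item name and itself, then destroys itself.
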(event `self.ReceiveBeginPlay`
  (`TextRenderComponent.K2_SetText` (`self.ItemName`) (`KismetTextLibrary.Conv_StringToText` (`self.Item Name`))))

(event `self.Sphere.OnComponentBeginOverlap`
  (params (OverlappedComponent :type "PrimitiveComponent Object Reference") (OtherActor :type "Actor Object Reference") (OtherComp :type "PrimitiveComponent Object Reference") (OtherBodyIndex :type Integer) (bFromSweep :type Boolean) (SweepResult :type "HitResult Structure (by ref)"))
  (if (`self.ActorHasTag` OtherActor "Player")
    (`self.OnItemPickup` (`self.Item Name`) self)
    (`self.K2_DestroyActor`)))

(fn `UserConstructionScript`)